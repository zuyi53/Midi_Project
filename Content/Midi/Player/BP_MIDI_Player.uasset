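; BP_MIDI_Player plays MIDI through a MIDI output device.
; It opens the output on BeginPlay, forwards every event from its Midi object to that device, and closes the output on EndPlay.
; As a temporary workaround when playback stops, it sends an event for every note on all 16 channels to silence the device.
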(event OnStop(Midi)
  (params (finished :type Boolean))
  ;[1 1 1] (temp Workaround) Stop All Midi
  (for _index (range 0 15)
    (for _index_2 (range 0 127)
      (Class|MidiInterface|SendMidiEvent (Utilities|Struct|MakeMidiEvent "MTE_NOTE" (Math|Conversions|ToByte(Integer) _index) (Math|Conversions|ToByte(Integer) _index_2) 0)))))

(event OnMidiEvent(Midi)
  (params (Event :type Midi%20Event%20Structure) (time :type Integer) (TrackID :type Integer))
  ;[1 1 1] Device Midi Synth
  (Class|MidiInterface|SendMidiEvent Event))

(event EventEndPlay
  (params (EndPlayReason :type EEndPlayReason%20Enum :default "Destroyed"))
  ;[1 1 1] Device Midi Synth
  (Class|MidiInterface|CloseMidiOutput))

(event EventBeginPlay
  ;[0 1 0.6045] Setup Midi
  (|CallParentFunction)
  ;[1 1 1] Device Midi Synth
  (Class|MidiInterface|OpenMidiOutput (Variables|Port|GetOutput)))

(fn ConstructionScript)