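; Actor component that visualizes MIDI note events as a row of colored cubes spawned at its owner's location.
; On BeginPlay it spawns half-scale BP_Visual_Box actors along Y, one per note when interfacing with a device, otherwise one per channel.
; Visualize picks the cube by note number or channel, setting a random color for note-on and black for note-off or zero velocity.
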(event Custom|Visualize
  (params (Event :type Midi%20Event%20Structure))
  ;[1 1 1] Check Events
  (if (or (Utilities|Enum|Equal(Enum) (.type Event) "MTE_NOTE") (== (.type Event) 8))
    ;[1 1 1] Visualization Cube
    (Default|SetColor (Utilities|Array|Get(acopy) (Variables|Default|GetVisual%20Cubes) (Math|Conversions|ToInteger(Byte) (select (Variables|Default|GetIs%20Interfacing) (.data1 Event) (.channel Event)))) (Math|Color|SelectColor :A (Math|Color|MakeColor (Math|Random|RandomFloat) (Math|Random|RandomFloat) (Math|Random|RandomFloat) 0.0) :bPickA (and (Utilities|Enum|Equal(Enum) (.type Event) "MTE_NOTE") (!= (.data2 Event) 0))))))

(event EventBeginPlay
  (bind _returnvalue (Components|GetOwner))
  (bind _returnvalue_2 (Transformation|GetActorLocation _returnvalue))
  ;[0.1194 0.5968 1] Create Visual Cubes
  (for _index (range 0 (select (Variables|Default|GetIs%20Interfacing) 127 15))
    (bind _returnvalue_3 (Game|SpawnActorfromClass "/Game/Midi/Other/BP_Visual_Box.BP_Visual_Box_C" (Math|Transform|MakeTransform (Math|Vector|MakeVector (.x _returnvalue_2) (+ (* _index 1e+02) (.y _returnvalue_2)) (.z _returnvalue_2)) "0, 0, 0" "0.500000,0.500000,0.500000") "AlwaysSpawn" 0 0))
    (Utilities|Array|Add (Variables|Default|GetVisual%20Cubes) _returnvalue_3)))