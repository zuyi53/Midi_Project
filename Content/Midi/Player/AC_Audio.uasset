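; Audio component for a MIDI player that turns note events into generated 2D tones.
; Play silences and destroys any sound at the slot indexed by channel × 16 + note, for both note-on and note-off.
; A nonzero-velocity note-on then spawns a fixed-amplitude constant tone at the note's frequency and stores it in that preallocated array.
; Stop mutes and destroys the stored sounds.
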(event Custom|Play
  (params (Event :type Midi%20Event%20Structure))
  (bind _returnvalue (Math|Conversions|ToInteger(Byte) (.channel Event)))
  (bind _returnvalue_2 (Math|Conversions|ToInteger(Byte) (.data1 Event)))
  (bind _2d_sound_items (Variables|Default|Get2D%20Sound%20Items))
  (bind _returnvalue_3 (* _returnvalue 16))
  (bind _returnvalue_4 (+ _returnvalue_3 _returnvalue_2))
  (bind _item (Utilities|Array|Get(acopy) _2d_sound_items _returnvalue_4))
  ;[0.09543 0.47 1] Check If Note Event
  (if (or (Utilities|Enum|Equal(Enum) (.type Event) "MTE_NOTE") (== (.type Event) 8))
    ;[1 0.008092 0] Play Multiple Audio
    (Utilities|FlowControl|Sequence
      (:then_0
        (Utilities|IsValid _item
          (:Is%20Valid
            (Audio|Components|Audio|SetVolumeMultiplier _item 0.0 :!class /Script/Engine.AudioComponent)
            (Components|DestroyComponent _item))))
      (:then_1
        (if (and (Utilities|Enum|Equal(Enum) (.type Event) "MTE_NOTE") (!= (.data2 Event) 0))
          (bind _returnvalue_5 (Class|SoundUtils|ConstantNote 2048.0 (Class|MidiUtils|NotetoFrequency (.data1 Event))))
          (bind _returnvalue_6 (Audio|SpawnSound2D _returnvalue_5 1.0 1.0))
          (Utilities|Array|SetArrayElem (Variables|Default|Get2D%20Sound%20Items) _returnvalue_4 _returnvalue_6))))))

(event Custom|Stop
  (bind _2d_sound_items (Variables|Default|Get2D%20Sound%20Items))
  ;[1 1 1] Stop Audio
  (Audio|Components|Audio|SetVolumeMultiplier _2d_sound_items 0.0 :!class /Script/Engine.AudioComponent)
  (Components|DestroyComponent _2d_sound_items))

(event EventBeginPlay
  (Utilities|Array|Resize (Variables|Default|Get2D%20Sound%20Items) 2048))