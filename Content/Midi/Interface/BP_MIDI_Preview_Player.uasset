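; Preview player Blueprint that plays a MIDI asset through a MIDI output and reports its notes.
; BeginPlay loads the asset and opens the output, then starts MidiAudio after a configurable delay; EndPlay closes the output.
; MidiAudio events are forwarded to the MIDI output.
; The Midi event handler filters note events (including type 8), prints channel, note and velocity, and dispatches the converted chord name.
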(event OnMidiEvent(Midi)
  (params (Event :type Midi%20Event%20Structure))
  ;[1 1 1] Device Midi Synth
  ;[1 0.4161 0.4062] Check Note Event
  (if (or (Utilities|Enum|Equal(Enum) (.type Event) "MTE_NOTE") (== (.type Event) 8))
    ;[1 1 1] DO anything like drawing to screen ext
    (Development|PrintString (Utilities|String|Append "Channel: " (Utilities|String|ToString(Byte) (.channel Event)) " Note: " (Utilities|String|ToString(Byte) (.data1 Event)) " Velocity: " (Utilities|String|ToString(Byte) (.data2 Event))))
    (Default|CallDispatchMidi (Utilities|String|EnumtoString (Class|MidiUtils|NotetoChord (.data1 Event))))))

(event OnEvent(MidiAudio)
  (params (Event :type Midi%20Event%20Structure))
  ;[1 1 1] Midi Audio
  (Class|MidiInterface|SendMidiEvent Event))

(event EventEndPlay
  (params (EndPlayReason :type EEndPlayReason%20Enum :default "Destroyed"))
  ;[1 1 1] Device Midi Synth
  (Class|MidiInterface|CloseMidiOutput))

(event EventBeginPlay
  ;[0 1 0.6045] Setup Midi Asset
  (Class|MidiComponent|LoadAsset (Variables|Default|GetMidi%20Audio) (Variables|Default|GetMidi%20Asset))
  (Class|MidiInterface|OpenMidiOutput (Variables|Default|GetOutput))
  (|CallParentFunction)
  ;[1 1 1] Setup and Play delay  Audio
  (Utilities|FlowControl|Delay (Variables|Default|GetDelay%20Sound%20Amount))
  (Class|MidiComponent|Start (Variables|Default|GetMidi%20Audio)))

(fn ConstructionScript)